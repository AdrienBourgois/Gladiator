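; Blood particle effect actor that leaves blood splat decals where its particles hit surfaces.
; Each particle collision passes its location and normal to SpawnBloodDecal, which orients a randomly sized decal along that normal.
; Every decal gets its own dynamic material instance with a random integer scalar, though the parameter name is set to None.
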(event OnParticleCollide(ParticleSystem)
  (params (EventName :type Name :default "None") (EmitterTime :type Float%20%28single-precision%29) (ParticleTime :type Integer) (Location :type Vector) (Velocity :type Vector :default "0, 0, 0") (Direction :type Vector :default "0, 0, 0") (Normal :type Vector) (BoneName :type Name :default "None"))
  (CallFunction|SpawnBloodDecal Location Normal))

(event EventBeginPlay)

(event Collision|EventActorBeginOverlap
  (params (OtherActor :type Actor%20Object%20Reference)))

(event EventTick
  (params (DeltaSeconds :type Float%20%28single-precision%29)))

(fn ConstructionScript)

(fn SpawnBloodDecal
  (params (Location :type Vector) (InVec :type Vector))
  (bind _returnvalue (Math|Random|RandomFloatinRange 1e+01 5e+01))
  (bind _returnvalue_2 (Rendering|Material|CreateDynamicMaterialInstance "/Game/Blueprints/ParticleSystem/BloodSplatMat.BloodSplatMat" :!class /Script/Engine.KismetMaterialLibrary))
  (Rendering|Material|SetScalarParameterValue _returnvalue_2 "None" (Math|Conversions|ToFloat(Integer) (Math|Random|RandomIntegerinRange 0 12)) :!class /Script/Engine.MaterialInstanceDynamic)
  (Rendering|Decal|SpawnDecalatLocation _returnvalue_2 (Math|Vector|MakeVector 1e+01 _returnvalue _returnvalue) Location (Math|Conversions|RotationFromXVector InVec) 0.0)
  (return))